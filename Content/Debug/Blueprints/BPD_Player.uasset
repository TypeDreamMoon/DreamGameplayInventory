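; BPD_Player is a debug player Blueprint for testing the Dream gameplay slot inventory.
; On BeginPlay it creates the debug slot inventory widget, adds it to the viewport and initializes it with the slot inventory component obtained from the first player state.
; Pressing 1 gives one debug single item by class to that inventory and prints the result.
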(event `self.ReceiveBeginPlay`
  (bind _returnvalue (`|CreateWidget` "/DreamGameplayInventory/Debug/SlotDebug/DW_Debug_SlotInventory.DW_Debug_SlotInventory_C"))
  (`UserWidget.AddToViewport` _returnvalue 0)
  (`/DreamGameplayInventory/Debug/SlotDebug/DW_Debug_SlotInventory.Initialize Widget` _returnvalue (`DreamGameplayInventoryBlueprintLibrary.AsDreamSlotInventoryComponent` (`DreamGameplayInventoryBlueprintLibrary.GetDreamGameplayInventory` (`GameplayStatics.GetPlayerState` 0)))))

(event `Key|One`
  (params (Key :type "Key Structure"))
  (:`Pressed`
    (bind _returnvalue (`DreamInventorySlotComponent.GiveItemByClass` (`DreamGameplayInventoryBlueprintLibrary.AsDreamSlotInventoryComponent` (`DreamGameplayInventoryBlueprintLibrary.GetDreamGameplayInventory` (`GameplayStatics.GetPlayerState` 0))) "/DreamGameplayInventory/Debug/Items/DIItem_Debug_Single.DIItem_Debug_Single_C" 1))
    (`KismetSystemLibrary.PrintString` (`KismetStringLibrary.Conv_IntToString` _returnvalue))))

(fn `UserConstructionScript`)